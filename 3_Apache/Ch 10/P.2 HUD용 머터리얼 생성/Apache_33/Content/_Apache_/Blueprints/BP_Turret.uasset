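; BP_Turret is an enemy anti-air turret that fires rocket pairs at the player's Apache helicopter.
; Tick aims the gun at the player, clamps pitch within search range, and shoots from both spawn points within fire range, throttled by a delay.
; The construction script gives each spawn point a slight random, opposing yaw.
; The first hit on the truck mesh marks it destroyed, increments BP_Apache's kill count and removes it after three seconds.
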(event OnComponentHit(Turret_Truck_DM)
  (params (HitComponent :type Primitive%20Component%20Object%20Reference) (OtherActor :type Actor%20Object%20Reference) (OtherComp :type Primitive%20Component%20Object%20Reference) (NormalImpulse :type Vector :default "0, 0, 0") (Hit :type Hit%20Result%20Structure%20%28by%20ref%29))
  ;[1 1 1] * 충돌처리..
  (Utilities|FlowControl|DoOnce false ; 1)  충돌 이벤트 발생시 단 1회만 처리..
    (:Completed
      (Variables|Default|SetisDestroyed true) ; 2)  isDestroy = true;
      (CallFunction|AddKillCount)
      (Utilities|FlowControl|Delay 3.0) ; 3)  3초간 다음 노드 처리 지연..
      (Actor|DestroyActor) ; 4)  액터 제거..
    )))

(event Custom|Shoot%20Bullet
  (bind _spawn_right (Variables|Default|GetSpawn%20Right))
  (bind _spawn_left (Variables|Default|GetSpawn%20Left))
  (bind _returnvalue (Transformation|GetWorldTransform _spawn_right))
  (bind _returnvalue_2 (Transformation|GetWorldTransform _spawn_left))
  ;[1 1 1] * 총알 발사
  (if (Variables|Default|GetcanFire) ; 1)  발사 가능한 상태인지 체크..
    (Variables|Default|SetcanFire false) ; 2)  포탄 발사 후 연속으로 발사되지 않도록 설정..
    (Game|SpawnActorfromClass "/Game/_Apache_/Blueprints/BP_Rocket_Enemy.BP_Rocket_Enemy_C" _returnvalue "Undefined" 0 0) ; 3)  [ BP_Rocket_Enemy ] 생성..
    (Effects|SpawnEmitteratLocation "/Game/_Apache_/Particles/P_Exp_1.P_Exp_1" (Math|Transform|TransformLocation _returnvalue "0, 0, 0")) ; 4)  화염 파티클 연출..
    (Game|SpawnActorfromClass "/Game/_Apache_/Blueprints/BP_Rocket_Enemy.BP_Rocket_Enemy_C" _returnvalue_2 "Undefined" 0 0)
    (Effects|SpawnEmitteratLocation "/Game/_Apache_/Particles/P_Exp_1.P_Exp_1" (Math|Transform|TransformLocation _returnvalue_2 "0, 0, 0"))
    ;;[1 1 1] 5)  발사후 일정시간( delay Time ) 동안 다음 발사 지연..
    (Utilities|FlowControl|Delay (Variables|Default|GetdelayTime))
    (Variables|Default|SetcanFire true)))

(event Custom|Build%20Dist%20Rot
  (bind _returnvalue (Game|Player|GetPlayerPawn 0))
  ;[1 1 1] * 헬기와의 거리와 방향 계산..
  ;;[1 1 1] 1) 포탑 -> 헬기로 향하는 방향 계산
  (Variables|Default|SettargetRotation (Math|Rotator|FindLookatRotation (Transformation|GetActorLocation) (Transformation|GetActorLocation _returnvalue)))
  ;;[1 1 1] 2)  거리 계산
  (Variables|Default|SettargetDist (Transformation|GetDistanceTo _returnvalue)))

(event Custom|Rotate%20Turret
  (bind _targetrotation (Variables|Default|GettargetRotation))
  (bind (_roll _pitch _yaw) (Math|Rotator|BreakRotator _targetrotation))
  ;[1 1 1] * 포탑 회전..
  ;;[1 1 1] 1)  현재 헬기와의 거리와 탐지거리 비교..
  (if (<= (Variables|Default|GettargetDist) (Variables|Default|GetsearchRange))
    ;;[1 1 1] 3)  포탑에 갱신된 회전값 적용..
    (Transformation|SetWorldRotation (Variables|Default|GetTurret_Gun_DM) (Math|Rotator|MakeRotator 0.0 (Math|Float|Clamp(Float) _pitch 0.0 4e+01) _yaw) false false)))

(event EventBeginPlay)

(event Collision|EventActorBeginOverlap
  (params (OtherActor :type Actor%20Object%20Reference)))

(event EventTick
  (params (DeltaSeconds :type Float%20%28single-precision%29))
  (Transformation|SetWorldRotation (Variables|Default|GetTurret_Gun_DM) (Math|Rotator|FindLookatRotation (Transformation|GetActorLocation) (Transformation|GetActorLocation (Game|Player|GetPlayerPawn 0))) false false) ; 4)  포탑을 3)의 회전값으로 회전
  ;[1 1 1] * 거리, 방향을 적용한 포탑 회전..
  (if (not (Variables|Default|GetisDestroyed))
    (CallFunction|BuildDistRot)
    (CallFunction|RotateTurret)
    (if (<= (Variables|Default|GettargetDist) (Variables|Default|GetfireRange))
      (CallFunction|ShootBullet))))

(fn ConstructionScript
  (bind _returnvalue (Math|Random|RandomFloatinRange 0.5 1.2))
  ;[1 1 1] 2)  1)의 값을 [ Yaw ] 회전으로
  ;       [ Spawn Left ]에 적용..
  (Transformation|SetRelativeRotation (Variables|Default|GetSpawn%20Left) (Math|Rotator|MakeRotator 0.0 0.0 _returnvalue) false false)
  ;[1 1 1] 3)  1)의 음수값을 [ Yaw ] 회전으로
  ;       [ Spawn Right ]에 적용..
  (Transformation|SetRelativeRotation (Variables|Default|GetSpawn%20Right) (Math|Rotator|MakeRotator 0.0 0.0 (* _returnvalue -1.0)) false false))

(fn AddKillCount
  ;[1 1 1] 1)   [ BP_Apache ] 참조..
  (bind _asbp_apache (Utilities|Casting|CastToBP_Apache (Game|Player|GetPlayerPawn 0)))
  (Default|AddKillCount _asbp_apache) ; 2)   KillCount를 1개 증가..
)