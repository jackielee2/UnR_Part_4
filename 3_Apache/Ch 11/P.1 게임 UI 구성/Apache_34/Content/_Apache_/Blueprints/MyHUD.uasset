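; MyHUD is a test HUD Blueprint that draws a horizontally centered test string near the top of the screen.
; DrawHUD stores the screen size each call, then DrawTextCenter measures the text width and uses GetCenterPos to compute the X position at a given Y.
; Disconnected nodes hold unused experiments with drawing text, materials and textures.
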(event EventBeginPlay)

(event Collision|EventActorBeginOverlap
  (params (OtherActor :type Actor%20Object%20Reference)))

(event EventTick
  (params (DeltaSeconds :type Float%20%28single-precision%29)))

(event EventDrawHUD
  (params (SizeX :type Integer) (SizeY :type Integer))
  ;[1 1 1] 화면 가운데( 너비만 적용 ) 문자열 출력하기..
  (CallFunction|SetScreenSize SizeX SizeY)
  (CallFunction|DrawTextCenter (Utilities|String|MakeLiteralString "HUD 테스트!!!") "(R=1.000000,G=1.000000,B=1.000000,A=1.000000)" 1e+02 "/Game/_Apache_/Fonts/MyFont.MyFont" 1.0))

(fn ConstructionScript)

(fn SetScreenSize
  (params (width :type Integer) (height :type Integer))
  (Variables|Default|SetScreenWidth (Math|Conversions|ToFloat(Integer) width))
  (Variables|Default|SetScreenHeight (Math|Conversions|ToFloat(Integer) height)))

(fn GetCenterPos
  (params (width :type Float%20%28single-precision%29))
  (return (* (- (Variables|Default|GetScreenWidth) width) 0.5)))

(fn DrawTextCenter
  (params (Text :type String) (Color :type Linear%20Color%20Structure) (ScreenY :type Float%20%28single-precision%29) (Font :type Font%20Object%20Reference) (Scale :type Float%20%28single-precision%29))
  (bind _result (CallFunction|GetCenterPos (.OutWidth (Class|HUD|GetTextSize Text Font Scale))))
  (HUD|DrawText Text Color _result ScreenY Font Scale false))