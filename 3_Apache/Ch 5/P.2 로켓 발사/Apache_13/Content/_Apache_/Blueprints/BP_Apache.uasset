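; BP_Apache is a player-controlled Apache helicopter that flies, turns and fires a pair of BP_Rockets from left and right arrow spawn points.
; Movement and yaw axes share an FInterpTo helper for eased, swept local offsets and rotation, with clamped roll banking the body in turns.
; Mouse axes drive clamped SpringArm pitch and yaw relative to the helicopter's heading.
; A timeline for spinning main and tail rotors exists but is never triggered.
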(event EventBeginPlay)

(event Collision|EventActorBeginOverlap
  (params (OtherActor :type Actor%20Object%20Reference)))

(event EventTick
  (params (DeltaSeconds :type Float%20%28single-precision%29)))

(event Input|ActionEvents|InputActionShoot
  (params (Key :type Key%20Structure :default "None"))
  (:Pressed
    (Utilities|FlowControl|Sequence ; 2)  시퀀스\n      - 연결된 노드들을 순서대로 처리
      (:then_0
        (Game|SpawnActorfromClass "/Game/_Apache_/Blueprints/BP_Rocket.BP_Rocket_C" (Transformation|GetWorldTransform (Variables|Default|GetArrow_SpawnR)) "Undefined" 0 0) ; 3)  spawn actor from class\n      -  [ Class ] 에 연결된 블루프린트를 참고하여 레벨에 액터를 생성.\n      -  [ Class ]   :   [ BP_Apache ]\n      -  [ Spawn Transform ]  :  액터를 생성할 때 참고할 트랜스폼 정보.
      )
      (:then_1
        (Game|SpawnActorfromClass "/Game/_Apache_/Blueprints/BP_Rocket.BP_Rocket_C" (Transformation|GetWorldTransform (Variables|Default|GetArrow_SpawnL)) "Undefined" 0 0)))))

(event Input|AxisEvents|InputAxisMoveForwardBack
  (params (AxisValue :type Float%20%28single-precision%29))
  (bind _return_value (CallFunction|MyInterpolation AxisValue (Variables|Default|GetCurrent%20X) (Variables|Default|GetMove%20Speed)))
  (Variables|Default|SetCurrent%20X _return_value) ; 선형보간 2)  보간된 값을 저장해서 다음 프레임때 활용한다.
  (Transformation|AddActorLocalOffset (Math|Vector|MakeVector _return_value 0.0 0.0) true false))

(event Input|AxisEvents|InputAxisMoveLeftRight
  (params (AxisValue :type Float%20%28single-precision%29))
  (bind _return_value (CallFunction|MyInterpolation AxisValue (Variables|Default|GetCurrent%20Y) (Variables|Default|GetMove%20Speed)))
  (Variables|Default|SetCurrent%20Y _return_value)
  (Transformation|AddActorLocalOffset (Math|Vector|MakeVector 0.0 _return_value 0.0) true false))

(event Input|AxisEvents|InputAxisMoveUpDown
  (params (AxisValue :type Float%20%28single-precision%29))
  (bind _return_value (CallFunction|MyInterpolation AxisValue (Variables|Default|GetCurrent%20Z) (Variables|Default|GetMove%20Speed)))
  (Variables|Default|SetCurrent%20Z _return_value)
  (Transformation|AddActorLocalOffset (Math|Vector|MakeVector 0.0 0.0 _return_value) true false))

(event Input|AxisEvents|InputAxisMouseRotUD
  (params (AxisValue :type Float%20%28single-precision%29))
  (CallFunction|ScrollUpDown AxisValue))

(event Input|AxisEvents|InputAxisRotate
  (params (AxisValue :type Float%20%28single-precision%29))
  (bind _return_value (CallFunction|MyInterpolation AxisValue (Variables|Default|GetCurrent%20Yaw) (Variables|Default|GetRot%20Speed)))
  (Variables|Default|SetCurrent%20Yaw _return_value)
  (Transformation|AddActorLocalRotation (Math|Rotator|MakeRotator 0.0 0.0 _return_value) true false)
  ;[1 1 1] ** 화면 기울이기 처리
  (bind _return_value_2 (CallFunction|MyInterpolation AxisValue (Variables|Default|GetArmRoll) 1.5e+03))
  (Variables|Default|SetArmRoll (Math|Float|Clamp(Float) _return_value_2 -15.0 15.0))
  (Transformation|SetWorldRotation (Variables|Default|GetBody) (Math|Rotator|MakeRotator (Variables|Default|GetArmRoll) 0.0 (.Yaw (Math|Rotator|BreakRotator (Transformation|GetActorRotation)))) true false) ; 4)  액터의 방향과 상관없이 회전량이 일정하므로 월드좌표로 회전연산
)

(event Input|AxisEvents|InputAxisMouseRotLR
  (params (AxisValue :type Float%20%28single-precision%29))
  (Variables|Default|SetArmYaw (Math|Float|Clamp(Float) (+ AxisValue (Variables|Default|GetArmYaw)) -8e+01 8e+01))
  (Transformation|SetWorldRotation (Variables|Default|GetSpringArm) (Math|Rotator|MakeRotator (Variables|Default|GetArmRoll) (Variables|Default|GetArmPitch) (+ (Variables|Default|GetArmYaw) (.Yaw (Math|Rotator|BreakRotator (Transformation|GetActorRotation))))) false false))

(fn ConstructionScript)

(fn MyInterpolation
  (params (Axis%20Value :type Float%20%28single-precision%29) (Current :type Float%20%28single-precision%29) (Speed :type Float%20%28single-precision%29))
  (bind _returnvalue (Utilities|Time|GetWorldDeltaSeconds))
  (return (Math|Interpolation|FInterpTo Current (* Axis%20Value Speed _returnvalue) _returnvalue 5.0)))

(fn ScrollUpDown
  (params (Axis%20Value :type Float%20%28single-precision%29))
  (Variables|Default|SetArmPitch (Math|Float|Clamp(Float) (+ Axis%20Value (Variables|Default|GetArmPitch)) -8e+01 3e+01))
  (Transformation|SetWorldRotation (Variables|Default|GetSpringArm) (Math|Rotator|MakeRotator (Variables|Default|GetArmRoll) (Math|Float|Clamp(Float) (+ Axis%20Value (Variables|Default|GetArmPitch)) -8e+01 3e+01) (+ (.Yaw (Math|Rotator|BreakRotator (Transformation|GetActorRotation))) (Variables|Default|GetArmYaw))) false false))