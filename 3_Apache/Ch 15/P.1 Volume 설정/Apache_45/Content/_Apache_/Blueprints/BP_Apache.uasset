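; Player Apache helicopter that fires twin rockets, with fuel drain, kill-count victory and game-over handling.
; Axis inputs use FInterpTo-smoothed movement, yaw and banking, plus boost, right-mouse camera orbit and a cockpit-view toggle.
; Tick drains Fuel, derives Hp from it and checks KillCount against EnemyCount.
; Widgets created via the Construction Script show HUD, pause and end menus; empty fuel or non-BlockingVolume collisions end the game.
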(event OnComponentHit(Body)
  (params (HitComponent :type Primitive%20Component%20Object%20Reference) (OtherActor :type Actor%20Object%20Reference) (OtherComp :type Primitive%20Component%20Object%20Reference) (NormalImpulse :type Vector :default "0, 0, 0") (Hit :type Hit%20Result%20Structure%20%28by%20ref%29))
  (bind _returnvalue (Utilities|GetDisplayName OtherActor))
  (Utilities|FlowControl|DoOnce false
    (:Completed
      ;[1 1 1] -  이름에 [ BlockingVolume ]이 포함되어 있는지 체크..
      (if (Utilities|String|Contains _returnvalue "BlockingVolume")
        (Development|PrintString "End Of Scene!!")
        (else
          (CallFunction|DestroySelf)
          (Development|PrintString (Utilities|String|Append "충돌한 오브젝트는 " _returnvalue " 입니다..")) ; 어떤 액터가 충돌했는지 디버깅 용으로 확인..
        )))))

(event EventBeginPlay
  (Utilities|FlowControl|Sequence
    (:then_0
      (Variables|Default|SetStart%20Speed (Variables|Default|GetMove%20Speed)) ; 1)   초기속도 설정..
    )
    (:then_1
      (UserInterface|Viewport|AddtoViewport (Variables|Default|GetGameUI) 0) ; [ Game UI ]위젯을 화면에 배치..
    )))

(event Collision|EventActorBeginOverlap
  (params (OtherActor :type Actor%20Object%20Reference)))

(event EventTick
  (params (DeltaSeconds :type Float%20%28single-precision%29))
  ;[1 1 1] * 게임 루프..
  (CallFunction|SetFuel)
  (CallFunction|SetHP)
  (CallFunction|CheckComplete))

(event Input|ActionEvents|InputActionShoot
  (params (Key :type Key%20Structure :default "None"))
  (bind _arrow_spawnr (Variables|Default|GetArrow_SpawnR))
  (bind _arrow_spawnl (Variables|Default|GetArrow_SpawnL))
  (bind _returnvalue (Transformation|GetWorldTransform _arrow_spawnr))
  (bind _returnvalue_2 (Transformation|GetWorldTransform _arrow_spawnl))
  (:Pressed
    (Utilities|FlowControl|Sequence ; 2)  시퀀스\n      - 연결된 노드들을 순서대로 처리
      (:then_0
        (Game|SpawnActorfromClass "/Game/_Apache_/Blueprints/BP_Rocket.BP_Rocket_C" _returnvalue "Undefined" 0 0) ; 3)  spawn actor from class\n      -  [ Class ] 에 연결된 블루프린트를 참고하여 레벨에 액터를 생성.\n      -  [ Class ]   :   [ BP_Apache ]\n      -  [ Spawn Transform ]  :  액터를 생성할 때 참고할 트랜스폼 정보.
        (Effects|SpawnEmitteratLocation "/Game/_Apache_/Particles/P_Exp_1.P_Exp_1" (Math|Transform|TransformLocation _returnvalue "0, 0, 0")))
      (:then_1
        (Game|SpawnActorfromClass "/Game/_Apache_/Blueprints/BP_Rocket.BP_Rocket_C" _returnvalue_2 "Undefined" 0 0)
        (Effects|SpawnEmitteratLocation "/Game/_Apache_/Particles/P_Exp_1.P_Exp_1" (Math|Transform|TransformLocation _returnvalue_2 "0, 0, 0"))))))

(event Input|ActionEvents|InputActionPopupMenu
  (params (Key :type Key%20Structure :default "None"))
  (:Pressed
    (Variables|Default|SetisPopup true)
    (CallFunction|ShowPopup)))

(event Input|ActionEvents|InputActionConvertView
  (params (Key :type Key%20Structure :default "None"))
  (bind _springarm (Variables|Default|GetSpringArm))
  (bind _cockpit (Variables|Default|GetCockpit))
  (:Pressed
    (Utilities|FlowControl|FlipFlop
      (:A
        (Variables|/Script/Engine.SpringArmComponent|SetTargetArmLength _springarm -2.5e+02)
        (UserInterface|Viewport|AddtoViewport _cockpit 0))
      (:B
        (Variables|/Script/Engine.SpringArmComponent|SetTargetArmLength _springarm 6e+02)
        (Widget|RemovefromParent _cockpit)))))

(event Input|AxisEvents|InputAxisMoveForwardBack
  (params (AxisValue :type Float%20%28single-precision%29))
  (bind _return_value (CallFunction|MyInterpolation AxisValue (Variables|Default|GetCurrent%20X) (Variables|Default|GetMove%20Speed)))
  (Variables|Default|SetCurrent%20X _return_value) ; 선형보간 2)  보간된 값을 저장해서 다음 프레임때 활용한다.
  (Transformation|AddActorLocalOffset (Math|Vector|MakeVector _return_value 0.0 0.0) true false))

(event Input|AxisEvents|InputAxisMoveLeftRight
  (params (AxisValue :type Float%20%28single-precision%29))
  (bind _return_value (CallFunction|MyInterpolation AxisValue (Variables|Default|GetCurrent%20Y) (Variables|Default|GetMove%20Speed)))
  (Variables|Default|SetCurrent%20Y _return_value)
  (Transformation|AddActorLocalOffset (Math|Vector|MakeVector 0.0 _return_value 0.0) true false))

(event Input|AxisEvents|InputAxisMoveUpDown
  (params (AxisValue :type Float%20%28single-precision%29))
  (bind _return_value (CallFunction|MyInterpolation AxisValue (Variables|Default|GetCurrent%20Z) (Variables|Default|GetMove%20Speed)))
  (Variables|Default|SetCurrent%20Z _return_value)
  (Transformation|AddActorLocalOffset (Math|Vector|MakeVector 0.0 0.0 _return_value) true false))

(event Input|AxisEvents|InputAxisMouseRotUD
  (params (AxisValue :type Float%20%28single-precision%29))
  (if (Variables|Default|GetIs%20Mouse%20RButton)
    (CallFunction|ScrollUpDown AxisValue)))

(event Input|AxisEvents|InputAxisRotate
  (params (AxisValue :type Float%20%28single-precision%29))
  (bind _return_value (CallFunction|MyInterpolation AxisValue (Variables|Default|GetCurrent%20Yaw) (Variables|Default|GetRot%20Speed)))
  (Variables|Default|SetCurrent%20Yaw _return_value)
  (Transformation|AddActorLocalRotation (Math|Rotator|MakeRotator 0.0 0.0 _return_value) true false)
  ;[1 1 1] ** 화면 기울이기 처리
  (bind _return_value_2 (CallFunction|MyInterpolation AxisValue (Variables|Default|GetArmRoll) 1.5e+03))
  (Variables|Default|SetArmRoll (Math|Float|Clamp(Float) _return_value_2 -15.0 15.0))
  (Transformation|SetWorldRotation (Variables|Default|GetBody) (Math|Rotator|MakeRotator (Variables|Default|GetArmRoll) 0.0 (.Yaw (Math|Rotator|BreakRotator (Transformation|GetActorRotation)))) true false) ; 4)  액터의 방향과 상관없이 회전량이 일정하므로 월드좌표로 회전연산
)

(event Input|AxisEvents|InputAxisMouseRotLR
  (params (AxisValue :type Float%20%28single-precision%29))
  (if (Variables|Default|GetIs%20Mouse%20RButton)
    (Variables|Default|SetArmYaw (Math|Float|Clamp(Float) (+ AxisValue (Variables|Default|GetArmYaw)) -8e+01 8e+01))
    (Transformation|SetWorldRotation (Variables|Default|GetSpringArm) (Math|Rotator|MakeRotator (Variables|Default|GetArmRoll) (Variables|Default|GetArmPitch) (+ (Variables|Default|GetArmYaw) (.Yaw (Math|Rotator|BreakRotator (Transformation|GetActorRotation))))) false false)
    (else
      (Transformation|AddActorLocalRotation (Math|Rotator|MakeRotator 0.0 0.0 AxisValue) false false)
      (bind _output_get (Variables|Default|SetArmRoll (Math|Float|Clamp(Float) (- (Variables|Default|GetArmRoll) (* AxisValue -1.0)) -15.0 15.0)))
      (Transformation|SetWorldRotation (Variables|Default|GetSpringArm) (Math|Rotator|MakeRotator _output_get (Variables|Default|GetArmPitch) (+ (.Yaw (Math|Rotator|BreakRotator (Transformation|GetActorRotation))) (Variables|Default|GetArmYaw))) false false))))

(event Input|AxisEvents|InputAxisBooster
  (params (AxisValue :type Float%20%28single-precision%29))
  (Variables|Default|SetMove%20Speed (+ (* AxisValue 1e+03) (Variables|Default|GetStart%20Speed))))

(event Input|MouseEvents|RightMouseButton
  (params (Key :type Key%20Structure :default "None"))
  (:Pressed
    (Variables|Default|SetIs%20Mouse%20RButton true))
  (:Released
    (Variables|Default|SetIs%20Mouse%20RButton false)))

(event Input|KeyboardEvents|Escape
  (params (Key :type Key%20Structure :default "None"))
  (:Pressed
    (Variables|Default|SetisPopup true)
    (CallFunction|ShowPopup)))

(fn ConstructionScript
  (CallFunction|CreateUI))

(fn MyInterpolation
  (params (Axis%20Value :type Float%20%28single-precision%29) (Current :type Float%20%28single-precision%29) (Speed :type Float%20%28single-precision%29))
  (bind _returnvalue (Utilities|Time|GetWorldDeltaSeconds))
  (return (Math|Interpolation|FInterpTo Current (* Axis%20Value Speed _returnvalue) _returnvalue 5.0)))

(fn ScrollUpDown
  (params (Axis%20Value :type Float%20%28single-precision%29))
  (Variables|Default|SetArmPitch (Math|Float|Clamp(Float) (+ Axis%20Value (Variables|Default|GetArmPitch)) -8e+01 3e+01))
  (Transformation|SetWorldRotation (Variables|Default|GetSpringArm) (Math|Rotator|MakeRotator (Variables|Default|GetArmRoll) (Math|Float|Clamp(Float) (+ Axis%20Value (Variables|Default|GetArmPitch)) -8e+01 3e+01) (+ (.Yaw (Math|Rotator|BreakRotator (Transformation|GetActorRotation))) (Variables|Default|GetArmYaw))) false false))

(fn AddKillCount
  (bind _result (Math|Integer|IncrementInt (Variables|Default|GetKillCount))
    (:%20%20
      (Development|PrintString (Utilities|String|ToString(Integer) _result)))))

(fn ChangeSound
  (Audio|Components|Audio|Stop (Variables|Default|GetBGM)) ; [ BGM ], [ Rotor Sound ] 재생 정지..
  (Audio|Components|Audio|Play (Variables|Default|GetGameover) 0.0) ; [ Game Over ] 재생..
)

(fn ShowCursor
  (params (isShow :type Boolean))
  (bind _returnvalue (Game|GetPlayerController 0))
  (if isShow
    ;[1 1 1] 입력 컨트롤 활성 / 비활성 처리..
    (Input|DisableInput _returnvalue)
    (else
      (Input|EnableInput _returnvalue)))
  (Variables|/Script/Engine.PlayerController|SetbShowMouseCursor _returnvalue isShow) ; 마우스 커서 노출 On / Off
  (Variables|/Script/Engine.PlayerController|SetbEnableClickEvents _returnvalue isShow) ; 클릭 이벤트 활성 On / Off
)

(fn ShowMenu
  (CallFunction|SetMenuTitle)
  (UserInterface|Viewport|AddtoViewport (Variables|Default|GetMain%20Menu) 0))

(fn SetDestroy
  (Variables|Default|SetisDead true)
  (Rendering|SetActorHiddenInGame true) ; 액터의 화면 표시여부 설정..
  (CallFunction|ChangeSound)
  (CallFunction|ShowCursor true)
  (CallFunction|ShowMenu)
  (Widget|RemovefromParent (Variables|Default|GetCockpit)))

(fn CheckComplete
  ;[1 1 1] 파괴한 대공포 수 >= 전체 대공포수 체크..
  (if (>= (Variables|Default|GetKillCount) (Variables|Default|GetEnemyCount))
    (Variables|Default|SetisComplete true)
    (CallFunction|ShowCursor true)
    (CallFunction|ShowMenu)))

(fn DestroySelf
  (bind _returnvalue (Transformation|GetActorLocation))
  (Variables|Default|SetisDead true)
  ;[1 1 1] 헬기의 위치에서 이펙트와 사운드 연출..
  (Effects|SpawnEmitteratLocation "/Game/_Apache_/Particles/P_Exp_2.P_Exp_2" _returnvalue)
  (Audio|PlaySoundatLocation "/Game/StarterContent/Audio/Explosion01.Explosion01" _returnvalue "0, 0, 0" 1.0 1.0 0.0 0 0 0)
  (CallFunction|SetDestroy))

(fn SetFuel
  (if (not (Math|Boolean|ORBoolean (Variables|Default|GetisDead) (Variables|Default|GetisComplete) (Variables|Default|GetisPopup)))
    ;[1 1 1] [ Fuel ]이 0 이하가 되면 [ Set Destroy ] 를 호출하여 게임 종료 처리..
    (bind _output_get (Variables|Default|Setfuel (- (Variables|Default|Getfuel) (* (Utilities|Time|GetWorldDeltaSeconds) 5e+01))))
    (if (< _output_get 0.0)
      (CallFunction|SetDestroy))))

(fn SetHP
  (Variables|Default|Sethp (Math|Float|Clamp(Float) (/ (Variables|Default|Getfuel) (Variables|Default|GetfuelMax)))))

(fn CreateUI
  (Utilities|FlowControl|Sequence
    (:then_0
      (bind _returnvalue (UserInterface|CreateWidget "/Game/_Apache_/Blueprints/_Widget/GameUI.GameUI_C")) ; [ 위젯 생성 ]\n - [ Class ]  :  [ Game UI ]
      (Variables|Default|SetGameUI _returnvalue) ; [ 변수로 승격 ]\n -  [ 이름 ]  :  [ GameUI ]\n -  [ Begin Play ]노드에서 UI를 화면에 생성하는데 사용..
    )
    (:then_1
      (bind _returnvalue_2 (UserInterface|CreateWidget "/Game/_Apache_/Blueprints/_Widget/MainMenu.MainMenu_C"))
      (Variables|Default|SetMain%20Menu _returnvalue_2))
    (:then_2
      (bind _returnvalue_3 (UserInterface|CreateWidget "/Game/_Apache_/Blueprints/_Widget/PopupMenu.PopupMenu_C"))
      (Variables|Default|SetPopup%20Menu _returnvalue_3))
    (:then_3
      (bind _returnvalue_4 (UserInterface|CreateWidget "/Game/_Apache_/Blueprints/_Widget/Cockpit.Cockpit_C"))
      (Variables|Default|SetCockpit _returnvalue_4))))

(fn SetMenuTitle
  (if (Variables|Default|GetisComplete)
    (bind _returnvalue (Appearance|GetDynamicMaterial (Variables|/Game/_Apache_/Blueprints/_Widget/MainMenu.MainMenu_C|GetMenuTitle (Variables|Default|GetMain%20Menu)) :!class /Script/UMG.Image)) ; 머터리얼 참조..
    (Rendering|Material|SetTextureParameterValue _returnvalue "TitleImage" "/Game/_Apache_/Textures/MissionComplete.MissionComplete") ; 텍스처 파라미터 설정..\n - 이미지 변경..
  ))

(fn ShowPopup
  (bind _popup_menu (Variables|Default|GetPopup%20Menu))
  (bind _returnvalue (Appearance|GetDynamicMaterial (Variables|/Game/_Apache_/Blueprints/_Widget/PopupMenu.PopupMenu_C|GetMenuTitle _popup_menu) :!class /Script/UMG.Image))
  (Rendering|Material|SetTextureParameterValue _returnvalue "TitleImage" "/Game/_Apache_/Textures/GamePause.GamePause")
  (UserInterface|Viewport|AddtoViewport _popup_menu 0)
  (CallFunction|ShowCursor true))