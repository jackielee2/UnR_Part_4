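; BP_Pickup is a fuel pickup for the Apache helicopter that plays a sound when collected.
; An overlap on its Pickup component checks the other actor's display name against "BP_Apache", then calls AddFuel.
; AddFuel casts player pawn 0 to BP_Apache, adds a fixed amount of fuel clamped to FuelMax, and destroys the pickup.
; An ItemRotation timeline drives actor yaw, but nothing in the graph starts it.
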(event OnComponentBeginOverlap(Pickup)
  (params (OverlappedComponent :type Primitive%20Component%20Object%20Reference) (OtherActor :type Actor%20Object%20Reference) (OtherComp :type Primitive%20Component%20Object%20Reference) (OtherBodyIndex :type Integer) (bFromSweep :type Boolean) (SweepResult :type Hit%20Result%20Structure%20%28by%20ref%29))
  (if (Utilities|Enum|Equal(Enum) (Utilities|GetDisplayName OtherActor) "BP_Apache")
    (CallFunction|AddFuel)
    (Audio|PlaySoundatLocation "/Game/_Apache_/Audios/PickupSound.PickupSound" (Transformation|GetActorLocation) "0, 0, 0" 1.0 1.0 0.0 0 0 0)))

(event EventBeginPlay)

(event Collision|EventActorBeginOverlap
  (params (OtherActor :type Actor%20Object%20Reference)))

(event EventTick
  (params (DeltaSeconds :type Float%20%28single-precision%29)))

(fn ConstructionScript)

(fn AddFuel
  ;[1 1 1] - 아이템 획득시 200 씩 [ Fuel ]에 추가..
  ; - 최대 연료( Fuel Max )를 초과하지 않도록 설정..( Clamp )
  ; - 헬기가 아이템 획득후 씬에서 제거..
  (bind _asbp_apache (Utilities|Casting|CastToBP_Apache (Game|Player|GetPlayerPawn 0)))
  (Variables|/Game/_Apache_/Blueprints/BP_Apache.BP_Apache_C|Setfuel _asbp_apache (Math|Float|Clamp(Float) (+ (Variables|/Game/_Apache_/Blueprints/BP_Apache.BP_Apache_C|Getfuel _asbp_apache) 2e+02) 0.0 (Variables|/Game/_Apache_/Blueprints/BP_Apache.BP_Apache_C|GetfuelMax _asbp_apache)))
  (Actor|DestroyActor))