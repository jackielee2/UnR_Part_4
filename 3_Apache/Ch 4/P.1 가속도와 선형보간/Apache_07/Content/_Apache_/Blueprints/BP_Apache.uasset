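; Apache helicopter Blueprint that moves forward and back along its local X axis from axis input.
; FInterpTo eases CurrentX toward the speed- and delta-time-scaled input, then is evaluated again on the updated value for a swept local offset.
; A RotationRotor timeline is set up to yaw the main rotor and pitch the tail rotor at double the angle, but nothing starts it.
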(event EventBeginPlay)

(event Collision|EventActorBeginOverlap
  (params (OtherActor :type Actor%20Object%20Reference)))

(event EventTick
  (params (DeltaSeconds :type Float%20%28single-precision%29)))

(event Input|AxisEvents|InputAxisMoveForwardBack
  (params (AxisValue :type Float%20%28single-precision%29))
  (bind _returnvalue (Utilities|Time|GetWorldDeltaSeconds))
  (Variables|Default|SetCurrent%20X (Math|Interpolation|FInterpTo (Variables|Default|GetCurrent%20X) (* AxisValue (Variables|Default|GetMove%20Speed) _returnvalue) _returnvalue 5.0)) ; 선형보간 2)  보간된 값을 저장해서 다음 프레임때 활용한다.
  (Transformation|AddActorLocalOffset (Math|Vector|MakeVector (Math|Interpolation|FInterpTo (Variables|Default|GetCurrent%20X) (* AxisValue (Variables|Default|GetMove%20Speed) _returnvalue) _returnvalue 5.0) 0.0 0.0) true false))

(fn ConstructionScript)