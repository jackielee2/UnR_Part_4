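; BP_Apache is an Apache helicopter actor that moves forward and backward from player input.
; The Move Forward Back axis drives a swept local X offset scaled by MoveSpeed and delta time, and prints the axis value for debugging.
; A RotationRotor timeline sets Rotor yaw and spins Tail pitch at twice that angle, though nothing in the graph triggers it.
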(event EventBeginPlay)

(event Collision|EventActorBeginOverlap
  (params (OtherActor :type Actor%20Object%20Reference)))

(event EventTick
  (params (DeltaSeconds :type Float%20%28single-precision%29)))

(event Input|AxisEvents|InputAxisMoveForwardBack
  (params (AxisValue :type Float%20%28single-precision%29))
  (Transformation|AddActorLocalOffset (Math|Vector|MakeVector (* AxisValue (Variables|Default|GetMove%20Speed) (Utilities|Time|GetWorldDeltaSeconds)) 0.0 0.0) true false) ; 5) 액터의 상대좌표를 기준으로 위치값을 누적\n     - Sweep \n          -  액터가 장애물에 충돌했을때 액터를 정지시키거나( On )\n              통과하도록 처리.( Off )\n          -  헬기가 지면이나 장애물을 뚫지 못하도록 [ On ]으로 처리.
  (Development|PrintString (Utilities|String|ToString(Float) AxisValue)))

(fn ConstructionScript)